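; Lever actor that lets the first-person player toggle a referenced jail bar open or closed.
; Its trigger volume enables input for player controller 0 when the FirstPersonCharacter overlaps it and disables input when it leaves.
; While input is enabled, pressing E flips the IsOpen flag on JailBarRef; any bar movement is left to that referenced object.
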(event `Key|E`
  ;[1 1 1] Trigger the Lever
  (:`Pressed`
    (if (`/Game/Blueprints/Jailbars.isOpen` (`self.JailBarRef`))
      (set `/Game/Blueprints/Jailbars.isOpen` false (`self.JailBarRef`))
      (else
        (set `/Game/Blueprints/Jailbars.isOpen` true (`self.JailBarRef`))))))

(event `self.Tigger.OnComponentBeginOverlap`
  (params (OtherActor :type "Actor Object Reference") (OtherComp :type "PrimitiveComponent Object Reference") (OtherBodyIndex :type Integer) (bFromSweep :type Boolean) (SweepResult :type "HitResult Structure (by ref)"))
  ;[1 1 1] Activate Inputs
  (cast `/Game/FirstPersonBP/Blueprints/FirstPersonCharacter` OtherActor)
  (`self.EnableInput` (`GameplayStatics.GetPlayerController` 0)))

(event `self.ReceiveBeginPlay`)

(event `self.Tigger.OnComponentEndOverlap`
  (params (OtherActor :type "Actor Object Reference") (OtherComp :type "PrimitiveComponent Object Reference") (OtherBodyIndex :type Integer))
  ;[1 1 1] Activate Inputs
  (cast `/Game/FirstPersonBP/Blueprints/FirstPersonCharacter` OtherActor)
  (`self.DisableInput` (`GameplayStatics.GetPlayerController` 0)))

(event `self.ReceiveActorBeginOverlap`
  (params (OtherActor :type "Actor Object Reference")))

(fn `UserConstructionScript`)