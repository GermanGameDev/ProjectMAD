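; Jail bars actor that the first-person character can open by holding E while standing in its trigger volume.
; Trigger overlap events enable and disable the actor's input for the player controller as the character enters and leaves.
; A timeline plays on press and reverses on release, moving the whole actor by a vector offset from its location stored at BeginPlay.
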(event `self.ReceiveActorBeginOverlap`
  (params (OtherActor :type "Actor Object Reference")))

(event `Key|E`
  (:`Pressed`
    (bind (_direction _jailbarsopen) (`Timeline|Timeline_0` :!label _label)
      (:`Update`
        (`self.K2_SetActorLocation` (`ActorComponent.GetOwner` (`self.JailBars`)) (+ _jailbarsopen (`self.JailbarsInitialLocation`)) false))))
  (:`Released`
    (goto _label :!via `Reverse`)))

(event `self.ReceiveActorEndOverlap`
  (params (OtherActor :type "Actor Object Reference")))

(event `self.Trigger.OnComponentBeginOverlap`
  (params (OtherActor :type "Actor Object Reference") (OtherComp :type "PrimitiveComponent Object Reference") (OtherBodyIndex :type Integer) (bFromSweep :type Boolean) (SweepResult :type "HitResult Structure (by ref)"))
  ;[1 1 1] Activate Inputs
  (cast `/Game/FirstPersonBP/Blueprints/FirstPersonCharacter` OtherActor)
  (`self.EnableInput` (`GameplayStatics.GetPlayerController` 0)))

(event `self.ReceiveBeginPlay`
  ;[1 1 1] Get Start Location
  (set `self.JailbarsInitialLocation` (`self.K2_GetActorLocation` (`ActorComponent.GetOwner` (`self.JailBars`)))))

(event `self.Trigger.OnComponentEndOverlap`
  (params (OtherActor :type "Actor Object Reference") (OtherComp :type "PrimitiveComponent Object Reference") (OtherBodyIndex :type Integer))
  ;[1 1 1] Activate Inputs
  (cast `/Game/FirstPersonBP/Blueprints/FirstPersonCharacter` OtherActor)
  (`self.DisableInput` (`GameplayStatics.GetPlayerController` 0)))

(fn `UserConstructionScript`)